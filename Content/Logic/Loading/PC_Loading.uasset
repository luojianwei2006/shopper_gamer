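; PC_Loading, apparently a player controller, drives the loading screen and opens the target level when loading completes.
; On BeginPlay it creates the loading widget, binds to the LoadingSubsystem's progress and completion delegates, and starts its LoadingPlan.
; Progress events update the widget's bar and percentage text, leaving the Status value unused.
; The completion event opens the reported level by name.
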(event Custom|进度变更
  (params (Percent :type Float%20%28single-precision%29) (Status :type Text))
  (bind __loadngui (Variables|Default|Get_LoadngUI))
  (Progress|SetPercent (Variables|/Game/Logic/Loading/UI/LoadingWidget.LoadingWidget_C|GetProgressBar_Progress __loadngui) Percent)
  (Rendering|Components|TextRender|SetText (Variables|/Game/Logic/Loading/UI/LoadingWidget.LoadingWidget_C|GetTextBlock_Progress __loadngui) (Utilities|Text|FormatText "{n}%" (* Percent 1e+02))))

(event Custom|进度完成
  (params (TargetLevel :type Name))
  (Game|OpenLevel(byName) TargetLevel))

(event EventBeginPlay
  (bind _returnvalue (Subsystems|GetLoadingSubsystem))
  (bind _returnvalue_2 (UserInterface|CreateWidget "/Game/Logic/Loading/UI/LoadingWidget.LoadingWidget_C"))
  (Variables|Default|Set_LoadngUI _returnvalue_2)
  (UserInterface|Viewport|AddtoViewport _returnvalue_2 0)
  (EventDispatchers|BindEventtoOnLoadingProgress _returnvalue (delegate Custom|进度变更))
  (EventDispatchers|BindEventtoOnLoadingComplete _returnvalue (delegate Custom|进度完成))
  (Class|LoadingSubsystem|StartLoading _returnvalue "/Game/Logic/LoadingPlan.LoadingPlan"))

(event EventTick
  (params (DeltaSeconds :type Float%20%28single-precision%29)))

(fn ConstructionScript)